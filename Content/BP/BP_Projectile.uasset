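; BP_Projectile is a projectile actor that travels along a direction supplied through its SetDirection event and expires after a fixed lifetime.
; Each Tick calls MoveComponentTo on the root, targeting the current location offset by direction times speed, with no hit or damage logic in the graph.
; A Delay on the same Tick destroys the actor after five seconds, and Destroyed spawns a scaled-down dark storm particle effect where it was.
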(event Custom|SetDirection
  (params (dir :type Vector))
  (Variables|Default|Setdirection dir))

(event EventTick
  (params (DeltaSeconds :type Float%20%28single-precision%29))
  (Utilities|FlowControl|Sequence
    (:then_0
      (Components|MoveComponentTo (Variables|Default|GetDefaultSceneRoot) (+ (* (Variables|Default|Getdirection) (Variables|Default|GetprojectileSpeed)) (Transformation|GetActorLocation)) "0, 0, 0" false false 0.2 false))
    (:then_1
      (Utilities|FlowControl|Delay 5.0)
      (Actor|DestroyActor))))

(event EventDestroyed
  (Effects|SpawnEmitteratLocation "/Game/FXVarietyPack/Particles/P_ky_darkStorm.P_ky_darkStorm" (Transformation|GetActorLocation) "0, 0, 0" "0.500000,0.500000,0.500000"))

(fn ConstructionScript)