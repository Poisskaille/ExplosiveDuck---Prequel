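; Interactable slot-machine actor that rolls five colored slots for a buff, though NewBuff is still an empty stub.
; Interact briefly locks use and animates the lever, then GenerateNumber rolls results with decreasing odds of extending a matching streak.
; SlotAnim cycles random materials, adding one slot per step through a state cascade, before FinalAnim shows the rolled result.
; The streak multiplier is returned but unused.
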(event Custom|AnimLever
  (bind _newtrack_0 (Timeline|LeverAnimTimeline PlayFromStart)
    (:Update
      (Transformation|SetRelativeRotation (Variables|Default|GetLevier) (Math|Rotator|MakeRotator (Math|Float|Lerp 0.0 1e+02 _newtrack_0) 0.0 0.0) false false))
    (:Finished
      (bind _buffvalue (CallFunction|GenerateNumber))
      (CallFunction|NewBuff _buffvalue)
      (Variables|Default|SetState "NewEnumerator0")
      (Variables|Default|SetloopIndex 0)
      (CallFunction|SlotAnim :!label _label)
      (Utilities|FlowControl|Delay 0.2)
      (Math|Integer|IncrementInt (Variables|Default|GetloopIndex)
        (:%20%20
          (if (>= (Variables|Default|GetloopIndex) 30)
            (Utilities|FlowControl|Delay 1.0)
            (CallFunction|FinalAnim)
            (else
              (goto _label))))))))

(event EventBeginPlay
  (bind _slotarray (Variables|Default|GetSlotArray))
  (bind _asbp_first_person_character (Utilities|Casting|CastToBP_FirstPersonCharacter (Game|GetPlayerCharacter 0)))
  (Variables|Default|SetCharacter _asbp_first_person_character)
  (Utilities|Array|Add _slotarray (Variables|Default|GetSlot1))
  (Utilities|Array|Add _slotarray (Variables|Default|GetSlot2))
  (Utilities|Array|Add _slotarray (Variables|Default|GetSlot3))
  (Utilities|Array|Add _slotarray (Variables|Default|GetSlot4))
  (Utilities|Array|Add _slotarray (Variables|Default|GetSlot5)))

(event EventInteract
  ;[1 1 1] Interaction
  (if (Variables|Default|GetisUsable)
    (Utilities|FlowControl|Sequence
      (:then_0
        (Variables|Default|SetisUsable false)
        (Utilities|FlowControl|Delay 0.5)
        (Variables|Default|SetisUsable true))
      (:then_1
        (CallFunction|AnimLever)))))

(fn ConstructionScript)

(fn NewBuff
  (params (Buff%20value :type Integer)))

(fn GenerateNumber
  (bind _returnvalue (Math|Random|RandomIntegerinRange 0 5))
  (bind _returnvalue_2 (Math|Random|RandomIntegerinRange 0 5))
  (bind _numberarray (Variables|Default|GetnumberArray))
  (CallFunction|ClearArray)
  (LocalVariables|Setstreak true)
  (bind _output_get (Variables|Default|SetfirstNumber (Math|Random|RandomIntegerinRange 0 5)))
  (LocalVariables|Set%25 85)
  (LocalVariables|SetstreakValue 0)
  (Utilities|Array|Add _numberarray _output_get)
  (for _index (range 1 4)
    (bind __ (CallFunction|GetPourcentage100))
    (if (and (<= __ (LocalVariables|Get%25)) (LocalVariables|Getstreak))
      (if (>= (LocalVariables|Get%25) 15)
        (LocalVariables|Set%25 (- (LocalVariables|Get%25) 35))
        (LocalVariables|Setstreak true)
        (Math|Integer|IncrementInt (LocalVariables|GetstreakValue)
          (:%20%20
            (Utilities|Array|Add _numberarray (Variables|Default|GetfirstNumber))))
        (elif (!= _returnvalue (Variables|Default|GetfirstNumber))
          (Utilities|Array|Add _numberarray (Variables|Default|GetfirstNumber))
          (else
            (Utilities|Array|Add _numberarray _returnvalue))))
      (else
        (LocalVariables|Setstreak false :!label _label)
        (if (!= _returnvalue_2 (Variables|Default|GetfirstNumber))
          (Utilities|Array|Add _numberarray _returnvalue_2)
          (else
            (goto _label))))))
  (for _array_element _numberarray
    (Development|PrintString (Utilities|String|ToString(Integer) _array_element)))
  (return _output_get (LocalVariables|GetstreakValue)))

(fn GetPourcentage100
  (return (Math|Random|RandomIntegerinRange 0 100)))

(fn ClearArray
  (Utilities|Array|Clear (Variables|Default|GetnumberArray)))

(fn SlotAnim
  (bind _returnvalue (Math|Random|RandomIntegerinRange 0 5))
  (switch Utilities|FlowControl|Switch|SwitchonEEAnimState (Variables|Default|GetState)
    (:NewEnumerator0
      (Variables|Default|SetState "NewEnumerator1"))
    (:NewEnumerator1
      (Variables|Default|SetState "NewEnumerator2")
      (bind _m_texture (CallFunction|GetMaterial _returnvalue :!label _label))
      (Rendering|Material|SetMaterial (Variables|Default|GetSlot2) 0 _m_texture))
    (:NewEnumerator2
      (Variables|Default|SetState "NewEnumerator3")
      (bind _m_texture_2 (CallFunction|GetMaterial _returnvalue :!label _label_2))
      (Rendering|Material|SetMaterial (Variables|Default|GetSlot3) 0 _m_texture_2)
      (goto _label))
    (:NewEnumerator3
      (Variables|Default|SetState "NewEnumerator4")
      (bind _m_texture_3 (CallFunction|GetMaterial _returnvalue :!label _label_3))
      (Rendering|Material|SetMaterial (Variables|Default|GetSlot4) 0 _m_texture_3)
      (goto _label_2))
    (:NewEnumerator4
      (bind _m_texture_4 (CallFunction|GetMaterial _returnvalue))
      (Rendering|Material|SetMaterial (Variables|Default|GetSlot5) 0 _m_texture_4)
      (goto _label_3)))
  (bind _m_texture_5 (CallFunction|GetMaterial _returnvalue))
  (Rendering|Material|SetMaterial (Variables|Default|GetSlot1) 0 _m_texture_5))

(fn GetMaterial
  (params (number :type Integer))
  (switch int number
    (:0
      (LocalVariables|SettextureSlot "/Game/Materials/M_White.M_White"))
    (:1
      (LocalVariables|SettextureSlot "/Game/Materials/M_Orange.M_Orange"))
    (:2
      (LocalVariables|SettextureSlot "/Game/Materials/M_Pink.M_Pink"))
    (:3
      (LocalVariables|SettextureSlot "/Game/Materials/M_Green.M_Green"))
    (:4
      (LocalVariables|SettextureSlot "/Game/Materials/M_Yellow.M_Yellow"))
    (:5
      (LocalVariables|SettextureSlot "/Game/Materials/M_Black.M_Black")))
  (return (LocalVariables|GettextureSlot)))

(fn FinalAnim
  (for (_array_element _array_index) (Variables|Default|GetnumberArray)
    (bind _m_texture (CallFunction|GetMaterial _array_element))
    (Rendering|Material|SetMaterial (Utilities|Array|Get(acopy) (Variables|Default|GetSlotArray) _array_index) 0 _m_texture))
  (Development|PrintString "Hello"))