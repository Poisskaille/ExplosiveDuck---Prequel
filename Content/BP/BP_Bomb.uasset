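; BP_Bomb is a bomb actor with a scaling cube progress bar that, once filled, leads to its destruction.
; StartIncrease shows the bar and grows Cube1's Y scale in a Delay loop, destroying the actor shortly after it reaches full.
; Stop reverses the loop to shrink the bar and hide it at zero.
; On Destroyed, it spawns a large explosion and awards experience to the player's BP_ThirdPersonCharacter.
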(event Custom|StartIncrease
  (bind _cube1 (Variables|Default|GetCube1))
  (bind _returnvalue (Transformation|GetWorldScale _cube1))
  (Rendering|SetVisibility (Variables|Default|GetCube) true true)
  (bind _output_get (Variables|Default|SetcanIncrease true))
  (if _output_get :!label _label
    (bind _output_get_2 (Variables|Default|SetsizeY (+ (Variables|Default|GetsizeY) 0.07)))
    (Transformation|SetWorldScale3D _cube1 (Math|Vector|MakeVector (.x _returnvalue) _output_get_2 (.z _returnvalue)))
    (Utilities|FlowControl|Delay 0.2)
    (if (>= (.y _returnvalue) 4.0)
      (Variables|Default|SetcanIncrease false)
      (Utilities|FlowControl|Delay 4.0)
      (Actor|DestroyActor)
      (else
        (goto _label)))))

(event Custom|Stop
  (bind _cube1 (Variables|Default|GetCube1))
  (bind _returnvalue (Transformation|GetWorldScale _cube1))
  (bind _output_get (Variables|Default|SetcanIncrease false))
  (if (not _output_get) :!label _label
    (bind _output_get_2 (Variables|Default|SetsizeY (+ (Variables|Default|GetsizeY) -0.07)))
    (Transformation|SetWorldScale3D _cube1 (Math|Vector|MakeVector (.x _returnvalue) _output_get_2 (.z _returnvalue)))
    (Utilities|FlowControl|Delay 0.2)
    (if (<= (.y _returnvalue) 0.0)
      (Rendering|SetVisibility (Variables|Default|GetCube) false true)
      (else
        (goto _label)))))

(event EventBeginPlay
  (Rendering|SetVisibility (Variables|Default|GetCube) false true))

(event EventDestroyed
  (Effects|SpawnEmitteratLocation "/Game/SFX/FXVarietyPack/Particles/P_ky_explosion.P_ky_explosion" (Transformation|GetWorldLocation (Variables|Default|GetStaticMesh)) "0, 0, 0" "5.000000,5.000000,5.000000")
  (bind _asbp_third_person_character (Utilities|Casting|CastToBP_ThirdPersonCharacter (Game|Player|GetPlayerPawn 0)))
  (Default|AddExp _asbp_third_person_character 5e+01))

(fn ConstructionScript)