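; Game mode that runs an object pool of BP_Enemy actors, pre-spawned at the BP_SpawnerEnemy location on BeginPlay.
; A looping timer activates pooled enemies from DeadEnemy by enabling collision and calling Spawn, and feeds the AliveEnemy list.
; Tick drives each alive enemy through CustomTick and prints both list sizes for debugging.
; DeleteEnemy recycles an enemy by disabling collision, moving it back to the spawner and returning it to the pool.
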(event EventBeginPlay
  (bind _returnvalue (Actor|GetActorOfClass "/Game/BP/EnemyIA/BP_SpawnerEnemy.BP_SpawnerEnemy_C"))
  (Variables|Default|SetspawnPos (Transformation|GetActorLocation _returnvalue))
  (Utilities|FlowControl|Sequence
    (:then_0
      (if (not (>= (Variables|Default|GetspawnEnemy) 150)) :!label _label
        (bind _returnvalue_2 (Game|SpawnActorfromClass "/Game/BP/EnemyIA/BP_Enemy.BP_Enemy_C" (Math|Transform|MakeTransform (Variables|Default|GetspawnPos) "0, 0, 0" "1.000000,1.000000,1.000000") "Undefined" "MultiplyWithRoot" 0 0))
        (CallFunction|RemoveCollider _returnvalue_2)
        (Utilities|Array|Add (Variables|Default|GetDeadEnemy) _returnvalue_2)
        (Math|Integer|IncrementInt (Variables|Default|GetspawnEnemy)
          (:%20%20
            (goto _label)))))
    (:then_1
      (Utilities|Time|SetTimerbyFunctionName 0 "SpawnEnnemy" 0.1 true))))

(event EventTick
  (params (DeltaSeconds :type Float%20%28single-precision%29))
  (Utilities|FlowControl|Sequence
    (:then_0
      (for _array_element (Variables|Default|GetAliveEnemy)
        (if (Utilities|IsValid _array_element)
          (Default|CustomTick _array_element))))
    (:then_2
      (Utilities|FlowControl|Delay 0.2)
      (Development|PrintString (Utilities|String|ToString(Integer) (Utilities|Array|Length (Variables|Default|GetDeadEnemy))) true true "(R=1.000000,G=0.085329,B=0.000000,A=1.000000)")
      (Development|PrintString (Utilities|String|ToString(Integer) (Utilities|Array|Length (Variables|Default|GetAliveEnemy))) true true "(R=0.000000,G=0.127423,B=1.000000,A=1.000000)"))))

(fn ConstructionScript)

(fn SpawnEnnemy
  (bind _deadenemy (Variables|Default|GetDeadEnemy))
  (bind _output (Utilities|Array|Get(acopy) _deadenemy))
  (if (> (Utilities|Array|Length _deadenemy) 0)
    (Utilities|IsValid _output
      (:Is%20Valid
        (CallFunction|EnableCollider _output)
        (Default|Spawn _output)
        (Utilities|Array|RemoveItem (Variables|Default|GetDeadEnemy) _output)
        (Utilities|Array|Add (Variables|Default|GetAliveEnemy) _output))
      (:Is%20Not%20Valid
        (Development|PrintString "OBJET INVALIDE !!!!!" true true "(R=0.044956,G=1.000000,B=0.000000,A=1.000000)")))))

(fn DeleteEnemy
  (params (Enemy :type BP%20Enemy%20Object%20Reference))
  (CallFunction|RemoveCollider Enemy)
  (Transformation|SetWorldLocation (Variables|/Script/Engine.Character|GetCapsuleComponent Enemy) (Variables|Default|GetspawnPos) false false)
  (Utilities|Array|RemoveItem (Variables|Default|GetAliveEnemy) Enemy)
  (Utilities|Array|Add (Variables|Default|GetDeadEnemy) Enemy))

(fn RemoveCollider
  (params (Enemy :type BP%20Enemy%20Object%20Reference))
  (Collision|SetCollisionProfileName (Variables|/Game/BP/EnemyIA/BP_Enemy.BP_Enemy_C|GetBox Enemy) "CustomNoCollide" true :!class /Script/Engine.PrimitiveComponent))

(fn EnableCollider
  (params (Enemy :type BP%20Enemy%20Object%20Reference))
  (Collision|SetCollisionProfileName (Variables|/Game/BP/EnemyIA/BP_Enemy.BP_Enemy_C|GetBox Enemy) "CustomCollide" true :!class /Script/Engine.PrimitiveComponent))