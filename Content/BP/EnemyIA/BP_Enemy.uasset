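; BP_Enemy is an enemy that chases the player and dies when projectile hits deplete its life.
; Every Tick it re-issues AIMoveTo toward player 0's BP_ThirdPersonCharacter pawn.
; A Box overlap with a BP_Projectile tagged "P" feeds its damage into CheckLife and destroys the projectile.
; CheckLife subtracts the damage from Life and reports depletion, upon which the enemy destroys itself.
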(event OnComponentBeginOverlap(Box)
  (params (OverlappedComponent :type Primitive%20Component%20Object%20Reference) (OtherActor :type Actor%20Object%20Reference) (OtherComp :type Primitive%20Component%20Object%20Reference) (OtherBodyIndex :type Integer) (bFromSweep :type Boolean) (SweepResult :type Hit%20Result%20Structure%20%28by%20ref%29))
  (if (Actor|ActorHasTag OtherActor "P")
    (bind _asbp_projectile (Utilities|Casting|CastToBP_Projectile OtherActor))
    (bind _isdead (CallFunction|CheckLife (Variables|/Game/BP/BP_Projectile.BP_Projectile_C|GetprojectileDamage _asbp_projectile)))
    (Actor|DestroyActor OtherActor)
    (if _isdead
      (Actor|DestroyActor))))

(event EventTick
  (params (DeltaSeconds :type Float%20%28single-precision%29))
  (bind _asbp_third_person_character (Utilities|Casting|CastToBP_ThirdPersonCharacter (Game|Player|GetPlayerPawn 0)))
  (AI|AIMoveTo self "0, 0, 0" _asbp_third_person_character 5.0 false))

(fn ConstructionScript)

(fn CheckLife
  (params (incomingDamage :type Integer))
  (bind _output_get (Variables|Default|Setlife (- (Variables|Default|Getlife) incomingDamage)))
  (return (<= _output_get 0)))